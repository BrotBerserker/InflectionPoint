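; Shield skill actor that makes its owner temporarily invincible.
; On BeginPlay it destroys itself if the owner's MortalityProvider reports not alive; otherwise it plays a spawn effect and sets that component's Invincible flag.
; After ShieldDuration it clears the flag if the owner is still valid, plays an explosion effect, removes the shield particles and destroys itself after a short delay.
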(event EventBeginPlay
  (bind _returnvalue (Components|GetOwner))
  (bind _returnvalue_2 (Actor|GetComponentbyClass _returnvalue "/Script/InflectionPoint.MortalityProvider"))
  (bind _returnvalue_3 (Class|MortalityProvider|IsAlive _returnvalue_2))
  (if _returnvalue_3
    (Effects|SpawnEmitterAttached "/Game/InflectionPoint/Effects/Skills/Shield/ShieldSpawn.ShieldSpawn" (Variables|Default|GetDefaultSceneRoot) "None" "-20.000000,0.000000,15.000000" "0, 0, 0" "2.000000,2.000000,2.000000")
    (Variables|/Script/InflectionPoint.MortalityProvider|SetInvincible _returnvalue_2 true)
    (Utilities|FlowControl|Delay (Variables|Default|GetShieldDuration))
    (Utilities|IsValid (Components|GetOwner)
      (:Is%20Valid
        (Variables|/Script/InflectionPoint.MortalityProvider|SetInvincible _returnvalue_2 false))
      (:Is%20Not%20Valid
        _))
    (Effects|SpawnEmitterAttached "/Game/InflectionPoint/Effects/Skills/Shield/ShieldExplosion.ShieldExplosion" (Variables|Default|GetDefaultSceneRoot) "None" "10.000000,0.000000,25.000000" "0, 0, 0" "0.500000,0.500000,0.500000")
    (Components|DestroyComponent (Variables|Default|GetShieldParticleSystem))
    (Utilities|FlowControl|Delay 0.5)
    (Actor|DestroyActor)
    (else
      (Actor|DestroyActor))))

(fn ConstructionScript)