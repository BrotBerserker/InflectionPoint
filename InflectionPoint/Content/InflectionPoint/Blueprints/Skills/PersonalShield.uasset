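; PersonalShield is a skill actor that makes its owning character temporarily invincible behind a shield effect.
; On BeginPlay it checks the owner's MortalityProvider, destroying itself if the owner is dead, otherwise granting timed invincibility with spawn particles and a looping sound.
; When the duration ends it fades the sound, explicitly clears invincibility, swaps the shield particles for an explosion, and destroys itself shortly after.
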(event EventBeginPlay
  (bind _returnvalue (Components|GetOwner))
  (bind _shieldduration (Variables|Default|GetShieldDuration))
  (bind _returnvalue_2 (Actor|GetComponentbyClass _returnvalue "/Script/InflectionPoint.MortalityProvider"))
  (bind _returnvalue_3 (Class|MortalityProvider|IsAlive _returnvalue_2))
  (if _returnvalue_3
    (Effects|SpawnEmitterAttached "/Game/InflectionPoint/Effects/Skills/Shield/ShieldSpawn.ShieldSpawn" (Variables|Default|GetDefaultSceneRoot) "None" "-20.000000,0.000000,15.000000" "0, 0, 0" "2.000000,2.000000,2.000000")
    (bind _returnvalue_4 (Audio|SpawnSoundAttached "/Game/InflectionPoint/Audio/ShieldLoopSound_Cue.ShieldLoopSound_Cue" (Variables|Transformation|GetRootComponent) "None" "0, 0, 0" "0, 0, 0" "KeepRelativeOffset" false 1.0 1.0 0.0 0 0))
    (Class|MortalityProvider|SetInvincibleforSeconds _returnvalue_2 _shieldduration)
    (Utilities|FlowControl|Delay _shieldduration)
    (Audio|Components|Audio|FadeOut _returnvalue_4 0.4 0.0 :!class /Script/Engine.AudioComponent)
    (Utilities|IsValid (Components|GetOwner)
      (:Is%20Valid
        (Variables|/Script/InflectionPoint.MortalityProvider|SetInvincible _returnvalue_2 false))
      (:Is%20Not%20Valid
        _))
    (Effects|SpawnEmitterAttached "/Game/InflectionPoint/Effects/Skills/Shield/ShieldExplosion.ShieldExplosion" (Variables|Default|GetDefaultSceneRoot) "None" "10.000000,0.000000,25.000000" "0, 0, 0" "0.500000,0.500000,0.500000")
    (Components|DestroyComponent (Variables|Default|GetShieldParticleSystem))
    (Utilities|FlowControl|Delay 0.5)
    (Actor|DestroyActor)
    (else
      (Actor|DestroyActor))))

(fn ConstructionScript)