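; TeleportCamera is a temporary camera actor that shows a transition toward the player's character, apparently for a teleport skill.
; On BeginPlay it becomes the PlayerController's view target and hides the character's third-person mesh.
; A timeline lerps it from StartLocation to the pawn's live location while rotating to face it.
; When close enough or the timeline finishes, it unhides the mesh, returns the view to the character and destroys itself.
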(event EventBeginPlay
  (bind _playercontroller (Variables|Default|GetPlayerController))
  (bind _returnvalue (Pawn|GetControlledPawn _playercontroller))
  (bind _returnvalue_2 (Transformation|GetActorLocation _returnvalue))
  (bind _asplayer_character_base (Utilities|Casting|CastToPlayerCharacterBase (Pawn|GetControlledPawn _playercontroller)))
  (Variables|Default|SetPlayerCharacter _asplayer_character_base)
  (Game|Player|SetViewTargetwithBlend (Variables|Default|GetPlayerController) self 0.0 "VTBlend_Linear" 0.0 false)
  (Development|SetHiddeninGame (Variables|/Script/InflectionPoint.BaseCharacter|GetMesh3P (Variables|Default|GetPlayerCharacter)) true false)
  (bind _newtrack_0 (Timeline|Timeline_0 Play)
    (:Update
      (Transformation|SetActorLocation (Math|Vector|Lerp(Vector) (Variables|Default|GetStartLocation) _returnvalue_2 _newtrack_0) false false)
      (Transformation|SetActorRotation (Math|Rotator|FindLookatRotation (Transformation|GetActorLocation) _returnvalue_2))
      (if (Math|Vector|Equal(Vector) _returnvalue_2 (Transformation|GetActorLocation) 3e+02)
        (Development|SetHiddeninGame (Variables|/Script/InflectionPoint.BaseCharacter|GetMesh3P (Variables|Default|GetPlayerCharacter)) false false :!label _label)
        (Game|Player|SetViewTargetwithBlend (Variables|Default|GetPlayerController) (Variables|Default|GetPlayerCharacter) 0.0 "VTBlend_Linear" 0.0 false)
        (Actor|DestroyActor)))
    (:Finished
      (goto _label))))

(fn ConstructionScript)