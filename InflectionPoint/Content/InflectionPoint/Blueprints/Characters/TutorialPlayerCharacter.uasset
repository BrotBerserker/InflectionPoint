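; Player character for the tutorial, layering tutorial-specific setup and death handling on a parent character.
; BeginPlay assigns the TDM player state to a fixed team, and possession registers the pawn with the TutorialPlayerController.
; When the MortalityProvider reports death, it shows the death camera, fires the multicast and client death calls, and stops the current weapon's tick.
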(event OnDeath(MortalityProvider)
  (params (KillingPlayer :type Controller%20Object%20Reference) (DamageCauser :type Actor%20Object%20Reference))
  (CallFunction|ShowDeathCamera)
  (Class|BaseCharacter|MulticastonDeath false)
  (Class|BaseCharacter|ClientonDeath)
  (Actor|Tick|SetActorTickEnabled (Variables|Default|GetCurrentWeapon)))

(event EventPossessed
  (params (NewController :type Controller%20Object%20Reference))
  (bind _astutorial_player_controller (Utilities|Casting|CastToTutorialPlayerController NewController))
  (Default|UpdateControlledPawn _astutorial_player_controller self))

(event EventBeginPlay
  (bind _astdmplayer_state_base (Utilities|Casting|CastToTDMPlayerStateBase (Variables|Default|GetPlayerState)))
  (Variables|/Script/InflectionPoint.TDMPlayerStateBase|SetTeam _astdmplayer_state_base 2))

(fn ConstructionScript
  (|CallParentFunction))