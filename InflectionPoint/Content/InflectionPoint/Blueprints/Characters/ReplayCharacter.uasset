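; Character that plays back a replay in a networked team deathmatch, with replay logic inherited or defined outside these graphs.
; On death it stops firing, multicasts the death, stops the replay and reports the kill to the TDM game mode.
; On the server, hitting or overlapping a Replay Breaker object switches off replay position correction.
; Tick pins the AI loading icon to a fixed world rotation.
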(event OnDeath(MortalityProvider)
  (params (KillingPlayer :type Controller%20Object%20Reference) (DamageCauser :type Actor%20Object%20Reference))
  (Class|BaseCharacter|ServerStopFire)
  (Class|BaseCharacter|MulticastonDeath)
  (Class|ReplayCharacterBase|StopReplay)
  (bind _astdmgame_mode_base (Utilities|Casting|CastToTDMGameModeBase (Game|GetGameMode)))
  (Class|TDMGameModeBase|CharacterDied _astdmgame_mode_base (Pawn|GetController) KillingPlayer DamageCauser))

(event OnComponentBeginOverlap(CapsuleComponent)
  (params (OverlappedComponent :type Primitive%20Component%20Object%20Reference) (OtherActor :type Actor%20Object%20Reference) (OtherComp :type Primitive%20Component%20Object%20Reference) (OtherBodyIndex :type Integer) (bFromSweep :type Boolean) (SweepResult :type Hit%20Result%20Structure%20%28by%20ref%29))
  (bind _disablescollision (Utilities|DisablesCorrection OtherComp))
  (if _disablescollision
    (Variables|Default|SetCorrectPositions false)))

(event OnComponentHit(CapsuleComponent)
  (params (HitComponent :type Primitive%20Component%20Object%20Reference) (OtherActor :type Actor%20Object%20Reference) (OtherComp :type Primitive%20Component%20Object%20Reference) (NormalImpulse :type Vector :default "0, 0, 0") (Hit :type Hit%20Result%20Structure%20%28by%20ref%29))
  (bind _disablescollision (Utilities|DisablesCorrection OtherComp))
  (if _disablescollision
    (Variables|Default|SetCorrectPositions false)))

(event EventTick
  (params (DeltaSeconds :type Float%20%28single-precision%29))
  (|CallParentFunction DeltaSeconds)
  (Transformation|SetWorldRotation (Variables|Default|GetLoadingAIIcon) "-90.000000, 0,90.000000" false false))

(fn ConstructionScript)

(fn CreateDynamicMaterial
  (params (Mesh :type Primitive%20Component%20Object%20Reference))
  (bind _returnvalue (Rendering|Material|CreateDynamicMaterialInstance Mesh 0 (Rendering|Material|GetMaterial Mesh 0) :!class /Script/Engine.PrimitiveComponent))
  (return _returnvalue))