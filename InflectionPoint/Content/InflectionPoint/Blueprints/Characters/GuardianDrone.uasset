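; Guardian drone character that rises from its spawn point on a timeline, then acts as an AI bot or replays a recorded run, depending on its instigator.
; Player-spawned drones record while botting and save to the player controller on destruction, keyed by phase and spawn time.
; Replay-spawned drones fetch that recording from the owning player and hand over to the AI when playback finishes.
; Death stops the replay and triggers an explosion.
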(event OnDeath(MortalityProvider)
  (params (KillingPlayer :type Controller%20Object%20Reference) (DamageCauser :type Actor%20Object%20Reference))
  (Class|BaseCharacter|MulticastonDeath false)
  (Class|ReplayCharacterBase|StopReplay)
  (CallFunction|DeathExplosion))

(event Custom|DeathExplosion
  (bind _returnvalue (Transformation|GetActorTransform))
  (bind _mesh3p (Variables|Default|GetMesh3P))
  (Rendering|SetCastShadow _mesh3p false)
  (Rendering|SetVisibility _mesh3p false false)
  (Collision|SetCollisionResponsetoAllChannels _mesh3p "ECR_Ignore")
  (Game|SpawnActorfromClass "/Game/InflectionPoint/Blueprints/Explosions/Fire_Explosion.Fire_Explosion_C" (Math|Transform|MakeTransform (.location _returnvalue) (.rotation _returnvalue) "2.000000,2.000000,2.000000") "AlwaysSpawn" 0 0)
  (Actor|SetLifeSpan 1.0))

(event Custom|OnFinishedReplaying_Event_0
  (bind _asguardian_drone_controller (Utilities|Casting|CastToGuardianDroneController (Pawn|GetController)))
  (Default|StartBotting _asguardian_drone_controller))

(event EventBeginPlay
  (bind _returnvalue (Transformation|GetActorLocation))
  (EventDispatchers|AssignOnFinishedReplaying (delegate Custom|OnFinishedReplaying_Event_0))
  (Audio|SpawnSoundAttached "/Game/InflectionPoint/Audio/SoundFX/Drone/DroneSpawn.DroneSpawn" (Variables|Default|GetCapsuleComponent) "None" "0, 0, 0" "0, 0, 0" "KeepRelativeOffset" false 1.0 1.0 0.0 0 0)
  (Utilities|FlowControl|Delay 0.1)
  (Rendering|SetVisibility (Variables|Default|GetMesh3P) true false)
  (bind _phase (CallFunction|GetPhase))
  (Variables|Default|SetCurrentPhase _phase)
  (bind _returnvalue_2 (Utilities|GetTimeSincePhaseStart))
  (Variables|Default|SetSpawnTime _returnvalue_2)
  (Utilities|InitializeAIController)
  ;[1 1 1] Start flying
  (Variables|Default|Setorigin%20location (Transformation|GetActorRotation))
  (Variables|Default|Setstartlocation _returnvalue)
  (Variables|Default|Settargetlocation (+ _returnvalue (* (Transformation|GetActorUpVector) 100)))
  (bind _newtrack_0 (Timeline|Timeline_0 PlayFromStart)
    (:Update
      (Transformation|SetActorLocationAndRotation (Math|Vector|Lerp(Vector) (Variables|Default|Getstartlocation) (Variables|Default|Gettargetlocation) _newtrack_0) (Math|Rotator|Lerp(Rotator) (Variables|Default|Getorigin%20location) (Math|Rotator|MakeRotator 0.0 0.0 (.yaw (Variables|Default|Getorigin%20location))) _newtrack_0)))
    (:Finished
      (bind _asguardian_drone_controller (Utilities|Casting|CastToGuardianDroneController (Pawn|GetController))) ; Only exists on the server
      (bind _replay_controller (Utilities|GetInstigatorController)
        (:IsPlayer
          (Class|PlayerStateRecorder|ServerStartRecording (Variables|Default|GetPlayerStateRecorder))
          (Default|StartBotting _asguardian_drone_controller))
        (:IsReplay
          (bind _asplayer_controller (Utilities|Casting|CastToPlayerController (Variables|/Script/InflectionPoint.AIControllerBase|GetOwningPlayerController _replay_controller)))
          (Utilities|Casting|CastToReplayCharacterBase (Pawn|GetControlledPawn _replay_controller))
          (bind _returnvalue_3 (Class|PlayerControllerBase|GetRecordedCharacterData _asplayer_controller "GuardianDrone_C" (Variables|Default|GetCurrentPhase) (Variables|Default|GetSpawnTime)))
          (Class|ReplayCharacterBase|SetReplayData _returnvalue_3)
          (Class|ReplayCharacterBase|StartReplay))))))

(event EventDestroyed
  (Networking|SwitchHasAuthority
    (:Authority
      (bind _asplayer_controller (Utilities|Casting|CastToPlayerController (Game|GetInstigatorController)))
      (Utilities|Array|Add (Variables|/Script/InflectionPoint.PlayerControllerBase|GetRecordedCharacterData _asplayer_controller) (Utilities|Struct|MakeRecordedCharacterData "GuardianDrone_C" (Variables|Default|GetCurrentPhase) (Variables|Default|GetSpawnTime) (Variables|/Script/InflectionPoint.PlayerStateRecorder|GetRecordedPlayerStates (Variables|Default|GetPlayerStateRecorder)))))))

(fn ConstructionScript)

(fn GetPhase
  (bind _asreplay_character_base (Utilities|Casting|CastToReplayCharacterBase (Game|GetInstigator))
    (:then
      (return (Variables|/Script/InflectionPoint.ReplayCharacterBase|GetReplayIndex _asreplay_character_base)))
    (:CastFailed
      (bind _astdmgame_state_base (Utilities|Casting|CastToTDMGameStateBase (Game|GetGameState)))
      (return (Variables|/Script/InflectionPoint.TDMGameStateBase|GetCurrentPhase _astdmgame_state_base)))))