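; Tutorial enemy character, an AI-controlled opponent that reacts to its own death.
; On BeginPlay it sets weapon 5 in its inventory to a single round of current ammo and sets third-person mesh custom depth from the VisibleThroughWalls flag.
; When the MortalityProvider reports death, it calls a multicast death event, then stops the AI controller's brain logic and movement if a valid brain component exists.
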(event OnDeath(MortalityProvider)
  (params (KillingPlayer :type Controller%20Object%20Reference) (DamageCauser :type Actor%20Object%20Reference))
  (bind _self self)
  (bind _returnvalue (AI|GetAIController _self))
  (bind _braincomponent (Variables|/Script/AIModule.AIController|GetBrainComponent _returnvalue))
  (Class|BaseCharacter|MulticastonDeath)
  (Utilities|IsValid _braincomponent
    (:Is%20Valid
      (AI|Logic|StopLogic _braincomponent "WTF")
      (AI|Navigation|StopMovement _returnvalue))))

(event EventBeginPlay
  (bind _returnvalue (Class|WeaponInventory|GetWeapon (Variables|Default|GetWeaponInventory) 5))
  (Variables|/Script/InflectionPoint.BaseWeapon|SetCurrentAmmo _returnvalue 1)
  (Rendering|SetRenderCustomDepth (Variables|Default|GetMesh3P) (Variables|Default|GetVisibleThroughWalls)))

(fn ConstructionScript)