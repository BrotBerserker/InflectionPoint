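; Player character Blueprint that connects initialization, death and directional damage events to its PlayerController and the game mode.
; On death, the server offsets the first-person camera as a death view, avoiding replication issues, stops the weapon and movement, and triggers client and multicast reactions.
; It reports the kill to the TDM game mode, then switches the spectated character after the death animation delay.
; Directional damage is forwarded to the controller on authority.
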(event OnDeath(MortalityProvider)
  (params (KillingPlayer :type Controller%20Object%20Reference) (DamageCauser :type Actor%20Object%20Reference))
  ;[1 1 1] Tell the GameMode that we died, do client-side stuff
  (CallFunction|ShowDeathCamera) ; Doing this on the server side to prevent camera replication issues
  (Class|BaseCharacter|ServerStopFire)
  (Actor|Tick|SetActorTickEnabled (Variables|Default|GetCurrentWeapon))
  (Class|BaseCharacter|ClientonDeath)
  (Class|BaseCharacter|MulticastonDeath)
  (bind _astdmgame_mode_base (Utilities|Casting|CastToTDMGameModeBase (Game|GetGameMode)))
  (Class|TDMGameModeBase|CharacterDied _astdmgame_mode_base (Pawn|GetController) KillingPlayer DamageCauser)
  (Variables|/Script/Engine.MovementComponent|SetVelocity (Pawn|GetMovementComponent) "0, 0, 0")
  (Utilities|FlowControl|Delay 2.5) ; Wait for death animation
  (bind _asplayer_controller (Utilities|Casting|CastToPlayerController (Pawn|GetController)))
  (Class|PlayerControllerBase|ServerSwitchSpectatedCharacter _asplayer_controller))

(event EventOnInitialized
  ;[1 1 1] Tell the controller that its character changed
  (bind _asplayer_controller (Utilities|Casting|CastToPlayerController (Pawn|GetController)))
  (Default|CharacterChanged _asplayer_controller self))

(event EventOnDirectionalDamageReceived
  (params (direction :type Vector :default "0, 0, 0") (damage :type Float%20%28single-precision%29) (DamageType :type Damage%20Type%20Class%20Reference))
  ;[1 1 1] Show Damage Dircetion
  (Networking|SwitchHasAuthority
    (:Authority
      (bind _asplayer_controller (Utilities|Casting|CastToPlayerController (Pawn|GetController)))
      (Default|DirectionalDamageReceived _asplayer_controller direction damage DamageType))))

(fn ConstructionScript)

(fn CreateDynamicMaterial
  (params (Mesh :type Primitive%20Component%20Object%20Reference))
  (bind _returnvalue (Rendering|Material|CreateDynamicMaterialInstance Mesh 0 (Rendering|Material|GetMaterial Mesh 0) :!class /Script/Engine.PrimitiveComponent))
  (return _returnvalue))

(fn ShowDeathCamera
  (Transformation|SetRelativeLocation (Variables|Default|GetFirstPersonCameraComponent) "-200.000000,1.750000,130.000000" false false))