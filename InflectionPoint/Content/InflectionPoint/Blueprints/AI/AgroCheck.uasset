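; AgroCheck is a behavior tree service that picks a visible target for a bot to follow.
; Each tick it clears TargetToFollow, then sphere-traces a large radius around the controlled pawn for desired object types, ignoring all BotCharacters.
; Camera-channel line traces confirm line of sight, and each visible hit overwrites TargetToFollow and TargetLocation, so the last one wins.
; TargetLocation is never cleared, so it retains the last seen position.
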(event EventTick
  (params (OwnerActor :type Actor%20Object%20Reference) (DeltaSeconds :type Float%20%28single-precision%29))
  (CallFunction|InitializeControllerReference OwnerActor)
  (Class|BTFunctionLibrary|SetBlackboardValueasObject (Variables|Default|GetTargetToFollow))
  (bind _outactors (Actor|GetAllActorsOfClass "/Game/InflectionPoint/Blueprints/Characters/BotCharacter.BotCharacter_C"))
  (bind _outhits (CallFunction|GetActorsinRange _outactors))
  (for _array_element _outhits
    (bind _hitactor (Utilities|IsVisible _array_element _outactors)
      (:true
        (CallFunction|SetTargettoFollow _hitactor)))))

(fn InitializeControllerReference
  (params (Object :type Object%20Object%20Reference))
  (Utilities|IsValid (Variables|Default|GetController)
    (:Is%20Not%20Valid
      (bind _asbot_controller (Utilities|Casting|CastToBotController Object))
      (Variables|Default|SetController _asbot_controller))))

(fn GetActorsinRange
  (params (ActorsToIgnore :type Array%20of%20Actor%20Object%20References))
  (bind _controller (Variables|Default|GetController))
  (bind _returnvalue (Pawn|GetControlledPawn _controller))
  (bind _returnvalue_2 (Transformation|GetActorLocation _returnvalue))
  (bind _output_get (Variables|Default|SetMyLocation _returnvalue_2))
  (bind _outhits (Collision|MultiSphereTraceForObjects _output_get (+ _returnvalue_2 "0, 0,15.000000") 1.5e+04 (Variables|Default|GetDesiredObjectTypes) false ActorsToIgnore "None"))
  (return _outhits))

(fn SetTargettoFollow
  (params (self2 :type Actor%20Object%20Reference))
  (Class|BTFunctionLibrary|SetBlackboardValueasObject (Variables|Default|GetTargetToFollow) self2)
  (AI|BehaviorTree|SetBlackboardValueasVector (Variables|Default|GetTargetLocation) (Transformation|GetActorLocation self2)))