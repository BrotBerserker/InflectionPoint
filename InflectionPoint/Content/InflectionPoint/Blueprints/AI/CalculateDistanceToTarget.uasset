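; Behavior tree node for the bot AI that keeps the distance to the current target up to date on the blackboard.
; On each tick it casts its owner to BotController and measures the straight-line distance between the controlled pawn and the blackboard Target actor.
; It writes the result to the DistanceToTarget key and also prints it as debug output.
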(event EventTick
  (params (OwnerActor :type Actor%20Object%20Reference) (DeltaSeconds :type Float%20%28single-precision%29))
  (bind _asbot_controller (Utilities|Casting|CastToBotController OwnerActor))
  (Variables|Default|SetController _asbot_controller)
  (Class|BTFunctionLibrary|SetBlackboardValueasFloat (Variables|Default|GetDistanceToTarget) (Math|Vector|VectorLength (- (Transformation|GetActorLocation (AI|BehaviorTree|GetBlackboardValueasActor (Variables|Default|GetTarget))) (Transformation|GetActorLocation (Pawn|GetControlledPawn (Variables|Default|GetController))))))
  (Development|PrintString (Utilities|String|ToString(Float) (Math|Vector|VectorLength (- (Transformation|GetActorLocation (AI|BehaviorTree|GetBlackboardValueasActor (Variables|Default|GetTarget))) (Transformation|GetActorLocation (Pawn|GetControlledPawn (Variables|Default|GetController))))))))