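; Behavior tree task that picks an AI character's weapon based on distance to its target.
; On tick, it walks the Weapons map, keyed by distance threshold, and takes the first key at or above the blackboard DistanceToTarget, so key order matters.
; It equips that weapon on the SelfActor BaseCharacter through ServerEquipSpecificWeapon, then finishes successfully, even when no threshold matches.
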(event EventTick
  (params (OwnerActor :type Actor%20Object%20Reference) (DeltaSeconds :type Float%20%28single-precision%29))
  (bind _asbase_character (Utilities|Casting|CastToBaseCharacter (AI|BehaviorTree|GetBlackboardValueasActor (Variables|Default|GetSelfActor))))
  (bind _keys (Utilities|Map|Keys (Variables|Default|GetWeapons)))
  (bind _array_element (Utilities|Array|ForEachLoopwithBreak _keys :!label _label)
    (:LoopBody
      (if (<= (Class|BTFunctionLibrary|GetBlackboardValueasFloat (Variables|Default|GetDistanceToTarget)) _array_element)
        (Class|BaseCharacter|ServerEquipSpecificWeapon _asbase_character (.Value (Utilities|Map|Find (Variables|Default|GetWeapons) _array_element)))
        (goto _label Break)))
    (:Completed
      (AI|BehaviorTree|FinishExecute true))))