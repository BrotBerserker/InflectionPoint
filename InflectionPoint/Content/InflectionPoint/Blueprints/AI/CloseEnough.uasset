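; Behavior tree decorator for bot AI that gates a branch on the bot's distance from the actor it follows.
; It casts the owner to BotController and measures from its controlled pawn to the TargetToFollow blackboard actor.
; Despite the CloseEnough name, the check passes when that distance is at least AcceptableDistance, meaning the target is not yet within range.
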(fn PerformConditionCheck
  (params (OwnerActor :type Actor%20Object%20Reference))
  (bind _asbot_controller (Utilities|Casting|CastToBotController OwnerActor))
  (Variables|Default|SetController _asbot_controller)
  (return (>= (Math|Vector|VectorLength (- (Transformation|GetActorLocation (AI|BehaviorTree|GetBlackboardValueasActor (Variables|Default|GetTargetToFollow))) (Transformation|GetActorLocation (Pawn|GetControlledPawn (Variables|Default|GetController))))) (Variables|Default|GetAcceptableDistance))))