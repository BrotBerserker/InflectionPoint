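; Jump pad actor that launches any BaseCharacter overlapping its trigger and plays a sound on every overlap.
; It can optionally zero the character's velocity and teleport them above the pad's origin before applying the impulse.
; CalculateImpulse builds the launch from forward and upward forces scaled by character mass, though it is applied as a velocity change.
; The construction script marks pads without positive directional force with an "x" text.
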(event OnComponentBeginOverlap(Trigger)
  (params (OverlappedComponent :type Primitive%20Component%20Object%20Reference) (OtherActor :type Actor%20Object%20Reference) (OtherComp :type Primitive%20Component%20Object%20Reference) (OtherBodyIndex :type Integer) (bFromSweep :type Boolean) (SweepResult :type Hit%20Result%20Structure%20%28by%20ref%29))
  (Audio|PlaySoundatLocation "/Game/InflectionPoint/Audio/JumpPadSound_Cue.JumpPadSound_Cue" (Transformation|GetActorLocation))
  (bind _asbase_character (Utilities|Casting|CastToBaseCharacter OtherActor))
  (Variables|InflectionPoint|SetCharacter _asbase_character)
  (if (Variables|InflectionPoint|GetIgnoreCharacterVelocity)
    (Utilities|ResetCharacterVelocity
      (:Out
        _)))
  (if (Variables|InflectionPoint|GetAdjustCharacterPosition)
    (Utilities|CenterCharacteronJumpPad
      (:Out
        _)))
  (Physics|AddImpulse (Variables|/Script/Engine.Character|GetCharacterMovement (Variables|InflectionPoint|GetCharacter)) (Utilities|CalculateImpulse (Variables|InflectionPoint|GetCharacter)) true))

(fn ConstructionScript
  (if (not (> (Variables|InflectionPoint|GetDirectionForce) 0.0))
    (Rendering|Components|TextRender|SetText (Actor|GetComponentbyClass "/Script/Engine.TextRenderComponent") (Utilities|Text|ToText(String) " x"))))