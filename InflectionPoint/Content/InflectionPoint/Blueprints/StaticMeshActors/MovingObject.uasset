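; MovingObject is an actor that moves a component back and forth along a spline at a set speed.
; Each Tick accumulates elapsed time, turns it into a ping-pong distance with modulo and absolute value, and places MovingComponent at that spline point in local space.
; An offset of one spline length makes the motion begin at the spline's start, and movement does not sweep for collision.
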(event EventBeginPlay)

(event Collision|EventActorBeginOverlap
  (params (OtherActor :type Actor%20Object%20Reference)))

(event EventTick
  (params (DeltaSeconds :type Float%20%28single-precision%29))
  (bind _spline (Variables|Default|GetSpline))
  (bind _returnvalue (Spline|GetSplineLength _spline))
  (Variables|Default|SetElapsedTime (+ DeltaSeconds (Variables|Default|GetElapsedTime)))
  (Transformation|SetRelativeLocation (Variables|Default|GetMovingComponent) (Spline|GetLocationatDistanceAlongSpline (Variables|Default|GetSpline) (Math|Float|Absolute(Float) (- (Math|Float|%(Float) (+ (* (Variables|Default|GetSpeed) (Variables|Default|GetElapsedTime)) _returnvalue) (* _returnvalue 2.0)) (Spline|GetSplineLength (Variables|Default|GetSpline)))) "Local") false false))

(fn ConstructionScript)