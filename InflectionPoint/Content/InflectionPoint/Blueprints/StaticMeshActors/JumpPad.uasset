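; Jump pad actor that launches any BaseCharacter entering its trigger and plays a sound on overlap.
; It optionally zeroes the character's velocity and teleports them above the pad, then applies a velocity-change impulse.
; The launch velocity comes from a suggested projectile arc toward ForceVector, with zero X nudged slightly.
; The construction script reuses that velocity to briefly draw the predicted trajectory as a preview.
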(event OnComponentBeginOverlap(Trigger)
  (params (OverlappedComponent :type Primitive%20Component%20Object%20Reference) (OtherActor :type Actor%20Object%20Reference) (OtherComp :type Primitive%20Component%20Object%20Reference) (OtherBodyIndex :type Integer) (bFromSweep :type Boolean) (SweepResult :type Hit%20Result%20Structure%20%28by%20ref%29))
  (Audio|PlaySoundatLocation "/Game/InflectionPoint/Audio/JumpPadSound_Cue.JumpPadSound_Cue" (Transformation|GetActorLocation) "0, 0, 0" 1.0 1.0 0.0 0 0 0)
  (bind _asbase_character (Utilities|Casting|CastToBaseCharacter OtherActor))
  (Variables|Default|SetCharacter _asbase_character)
  (if (Variables|Default|GetIgnoreCharacterVelocity)
    (Utilities|ResetCharacterVelocity
      (:Out
        _)))
  (if (Variables|Default|GetAdjustCharacterPosition)
    (Utilities|CenterCharacteronJumpPad
      (:Out
        _)))
  (bind _impuls (Utilities|CalcImpuls)
    (:Out
      (Physics|AddImpulse (Variables|/Script/Engine.Character|GetCharacterMovement (Variables|Default|GetCharacter)) _impuls true))))

(fn ConstructionScript
  (bind _impuls (Utilities|CalcImpuls)
    (:Out
      (Class|GameplayStatics|BlueprintPredictProjectilePathbyObjectType (+ (Transformation|GetActorLocation) "0, 0,10.000000") _impuls true 2.0 (Utilities|Array|MakeArray "ObjectTypeQuery1") false 0 "ForDuration" 0.1))))