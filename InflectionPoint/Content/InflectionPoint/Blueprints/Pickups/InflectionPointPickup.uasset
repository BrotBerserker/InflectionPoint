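; A pickup spawner that shows a timed countdown, then spawns an InflectionPoint actor at its IPPosition component.
; On BeginPlay a timeline starts, and its rounded track value updates the text render each tick.
; When the timeline finishes, only the authority spawns the actor, sets its tags to "None" and clears the text.
; The spawn happens once, with no restart of the countdown.
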(event EventBeginPlay
  (bind _newtrack_0 (Timeline|Timeline_0 PlayFromStart)
    (:Update
      (Rendering|Components|TextRender|SetText (Variables|Default|GetTextRender) (Utilities|Text|ToText(Integer) (Math|Float|Round _newtrack_0))))
    (:Finished
      (Networking|SwitchHasAuthority
        (:Authority
          (bind _returnvalue (Game|SpawnActorfromClass "/Game/InflectionPoint/Blueprints/Pickups/InflectionPoint.InflectionPoint_C" (Transformation|GetWorldTransform (Variables|Default|GetIPPosition)) "AlwaysSpawn" 0 0))
          (Variables|/Script/Engine.Actor|SetTags _returnvalue (Utilities|Array|MakeArray "None"))
          (Rendering|Components|TextRender|SetText (Variables|Default|GetTextRender) (Utilities|Text|MakeLiteralText "")))))))

(fn ConstructionScript)