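; AmmoPickup is a pickup that adds ammo to an interacting character's weapon of a configured type, if that character's inventory has one.
; On success it calls ServerIncreaseCurrentAmmo on the weapon, then hides the HoverRotator hierarchy for a short fixed delay before showing it again, toggling only visibility.
; The construction script picks the display mesh from a map keyed by weapon type, falling back to a bush mesh.
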(event EventOnCharacterInteract
  (params (Character :type Base%20Character%20Object%20Reference))
  (bind _hoverrotator (Variables|Default|GetHoverRotator))
  (bind _returnvalue (Class|WeaponInventory|GetWeaponbyClass (Variables|/Script/InflectionPoint.BaseCharacter|GetWeaponInventory Character) (Variables|Default|GetWeaponType)))
  (Utilities|IsValid _returnvalue
    (:Is%20Valid
      (Class|BaseWeapon|ServerIncreaseCurrentAmmo _returnvalue (Variables|Default|GetAmmoAmount))
      (Rendering|SetVisibility _hoverrotator false true)
      (Utilities|FlowControl|Delay 3.0)
      (Rendering|SetVisibility _hoverrotator true true))))

(fn ConstructionScript
  (bind _ammomesh_0 (Variables|Default|GetAmmoMesh_0))
  (bind _weaponpickupmeshes (Variables|Default|GetWeaponPickupMeshes))
  (bind _weapontype (Variables|Default|GetWeaponType))
  (bind (_value _returnvalue) (Utilities|Map|Find _weaponpickupmeshes _weapontype))
  (if _returnvalue
    (Components|StaticMesh|SetStaticMesh _ammomesh_0 _value)
    (else
      (Components|StaticMesh|SetStaticMesh _ammomesh_0 "/Game/StarterContent/Props/SM_Bush.SM_Bush"))))