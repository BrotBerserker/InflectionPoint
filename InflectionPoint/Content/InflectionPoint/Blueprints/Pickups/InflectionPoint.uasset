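; Team-colored Inflection Point pickup that awards one IP point to the collecting player.
; On spawn it takes the instigator's team, tints its particles, ignores movement collision with the instigator and enables overlaps after a short delay.
; Only non-replay characters of the matching team, or any team when Team is 0, can collect it.
; Collection updates PlayerState, notifies the controller, attaches sound and effects to the collector, then deactivates and expires.
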(event OnComponentBeginOverlap(Sphere)
  (params (OverlappedComponent :type Primitive%20Component%20Object%20Reference) (OtherActor :type Actor%20Object%20Reference) (OtherComp :type Primitive%20Component%20Object%20Reference) (OtherBodyIndex :type Integer) (bFromSweep :type Boolean) (SweepResult :type Hit%20Result%20Structure%20%28by%20ref%29))
  (bind _rootcomponent (Variables|/Script/Engine.Actor|GetRootComponent OtherActor))
  (Utilities|IsinCorrectTeam OtherActor
    (:True
      (CallFunction|IncreaseIPs OtherActor)
      (Audio|SpawnSoundAttached "/Game/InflectionPoint/Audio/IPEffect_Cue.IPEffect_Cue" _rootcomponent "None" "0, 0, 0" "0, 0, 0" "KeepRelativeOffset" false 1.0 1.0 0.0 0 0)
      (bind _returnvalue (Effects|SpawnEmitterAttached "/Game/InflectionPoint/Effects/InflectionPointPickup.InflectionPointPickup" _rootcomponent "None" "0, 0,-80.000000" "0,180.000000, 0"))
      (CallFunction|ApplyTeamColor _returnvalue)
      (CallFunction|Die))))

(event EventBeginPlay
  (CallFunction|SaveTeam)
  (CallFunction|ApplyTeamColor (Variables|Emitter|GetParticleSystemComponent))
  (CallFunction|ApplyTeamColor (Variables|Default|GetInflectionPointIdle))
  (CallFunction|IgnoreInstigator)
  (Utilities|FlowControl|Delay 2.0)
  (Variables|/Script/Engine.PrimitiveComponent|SetbGenerateOverlapEvents (Variables|Default|GetSphere) true))

(event EventTick
  (params (DeltaSeconds :type Float%20%28single-precision%29))
  (CallFunction|Rotate DeltaSeconds))

(fn ConstructionScript)

(fn ApplyTeamColor
  (params (ParticleSystem :type Particle%20System%20Component%20Object%20Reference))
  (Utilities|IsValid ParticleSystem
    (:Is%20Valid
      (bind _astdmgame_state_base (Utilities|Casting|CastToTDMGameStateBase (Game|GetGameState)))
      (Effects|Components|ParticleSystem|SetVectorParameter ParticleSystem "Supercolor" (* (Math|Conversions|ToVector(LinearColor) (Math|Conversions|ToLinearColor(Color) (Utilities|Array|Get(acopy) (Variables|/Script/InflectionPoint.TDMGameStateBase|GetTeamColors _astdmgame_state_base) (Variables|Default|GetTeam)))) 3e+02)))))

(fn IgnoreInstigator
  (bind _returnvalue (Game|GetInstigator))
  (Collision|IgnoreActorwhenMoving (Variables|Default|GetSphere) _returnvalue true)
  (bind _asbase_character (Utilities|Casting|CastToBaseCharacter _returnvalue))
  (Collision|IgnoreActorwhenMoving (Variables|/Script/Engine.Character|GetCapsuleComponent _asbase_character) self true))

(fn Rotate
  (params (DeltaSeconds :type Float%20%28single-precision%29))
  (bind _particlesystemcomponent (Variables|Emitter|GetParticleSystemComponent))
  (bind _returnvalue (Transformation|GetWorldRotation _particlesystemcomponent))
  (bind (_roll _pitch _yaw) (Math|Rotator|BreakRotator _returnvalue))
  (Utilities|IsValid _particlesystemcomponent
    (:Is%20Valid
      (Transformation|SetWorldRotation _particlesystemcomponent (Math|Rotator|MakeRotator _roll _pitch (+ _yaw (* DeltaSeconds 4e+01))) false false))))

(fn IncreaseIPs
  (params (Actor :type Object%20Object%20Reference))
  (bind _asbase_character (Utilities|Casting|CastToBaseCharacter Actor))
  (bind _asplayer_controller (Utilities|Casting|CastToPlayerController (Pawn|GetController _asbase_character)))
  (Default|DisplayInflectionPointCollected _asplayer_controller)
  (bind _astdmplayer_state_base (Utilities|Casting|CastToTDMPlayerStateBase (Variables|/Script/Engine.Pawn|GetPlayerState _asbase_character)))
  (Variables|/Script/InflectionPoint.TDMPlayerStateBase|SetIPPoints _astdmplayer_state_base (+ (Variables|/Script/InflectionPoint.TDMPlayerStateBase|GetIPPoints _astdmplayer_state_base) 1)))

(fn Die
  (Components|Activation|Deactivate (Variables|Emitter|GetParticleSystemComponent))
  (Variables|/Script/Engine.PrimitiveComponent|SetbGenerateOverlapEvents (Variables|Default|GetSphere) false)
  (Actor|SetLifeSpan 2.0))

(fn SaveTeam
  (bind _returnvalue (Game|GetInstigator))
  (Utilities|IsValid _returnvalue
    (:Is%20Valid
      (bind _returnvalue_2 (Class|CharacterInfoProvider|GetCharacterInfo (Actor|GetComponentbyClass _returnvalue "/Script/InflectionPoint.CharacterInfoProvider")))
      (Variables|Default|SetTeam (.Team (Utilities|Struct|BreakCharacterInfo _returnvalue_2))))))