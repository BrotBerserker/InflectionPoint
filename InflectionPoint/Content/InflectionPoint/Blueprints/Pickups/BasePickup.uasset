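; Base pickup actor that hovers, spins and reacts when a character touches it.
; Tick moves the HoverRotator component up and down between two height limits, flipping a direction flag at each end, while steadily yawing it.
; When a BaseCharacter overlaps the Trigger, it plays the pickup sound and calls OnCharacterInteract, an empty event that serves as a hook for the actual pickup effect.
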(event OnComponentBeginOverlap(Trigger)
  (params (OverlappedComponent :type Primitive%20Component%20Object%20Reference) (OtherActor :type Actor%20Object%20Reference) (OtherComp :type Primitive%20Component%20Object%20Reference) (OtherBodyIndex :type Integer) (bFromSweep :type Boolean) (SweepResult :type Hit%20Result%20Structure%20%28by%20ref%29))
  (bind _asbase_character (Utilities|Casting|CastToBaseCharacter OtherActor))
  (Utilities|IsValid _asbase_character
    (:Is%20Valid
      (Audio|PlaySoundatLocation (Variables|Default|GetPickUpSound) (Transformation|GetActorLocation) "0, 0, 0" 1.0 1.0 0.0 0 0 0)
      (CallFunction|OnCharacterInteract _asbase_character))))

(event Custom|OnCharacterInteract
  (params (Character :type Base%20Character%20Object%20Reference)))

(event EventTick
  (params (DeltaSeconds :type Float%20%28single-precision%29))
  (bind _hoverrotator (Variables|Default|GetHoverRotator))
  (bind _hoverrotator_2 (Variables|Default|GetHoverRotator))
  (bind _relativelocation (Variables|/Script/Engine.SceneComponent|GetRelativeLocation _hoverrotator))
  (bind _relativelocation_2 (Variables|/Script/Engine.SceneComponent|GetRelativeLocation _hoverrotator_2))
  (bind (_x _y) (Math|Vector|BreakVector _relativelocation))
  (bind _z (Math|Vector|BreakVector _relativelocation_2))
  (Transformation|SetRelativeTransform (Variables|Default|GetHoverRotator) (Math|Transform|MakeTransform (+ _relativelocation (Math|Vector|MakeVector _x _y (* (select (Variables|Default|GetMovingUp) 1.0 -1.0) DeltaSeconds 7.0))) (Math|Rotator|CombineRotators (Variables|/Script/Engine.SceneComponent|GetRelativeRotation _hoverrotator) (Math|Rotator|MakeRotator 0.0 0.0 (* DeltaSeconds 1e+02))) (Variables|/Script/Engine.SceneComponent|GetRelativeScale3D _hoverrotator)) false false)
  (if (>= _z 1e+01)
    (Variables|Default|SetMovingUp false)
    (elif (<= _z 0.0)
      (Variables|Default|SetMovingUp true))))

(fn ConstructionScript)