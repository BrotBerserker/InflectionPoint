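; DummyAmmoPickup is a pickup Blueprint that only animates an ammo mesh, with no collection or ammo logic.
; Each Tick spins AmmoMesh around yaw and bobs it along Z at a steady, frame-rate-independent speed, flipping the MovingUp flag at fixed height limits.
; The location update also adds the mesh's relative X and Y to themselves, so any non-zero horizontal offset doubles every frame.
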(event EventTick
  (params (DeltaSeconds :type Float%20%28single-precision%29))
  (bind _ammomesh (Variables|Default|GetAmmoMesh))
  (bind _ammomesh_2 (Variables|Default|GetAmmoMesh))
  (bind _relativelocation (Variables|/Script/Engine.SceneComponent|GetRelativeLocation _ammomesh))
  (bind _relativelocation_2 (Variables|/Script/Engine.SceneComponent|GetRelativeLocation _ammomesh_2))
  (bind (_x _y) (Math|Vector|BreakVector _relativelocation))
  (bind _z (Math|Vector|BreakVector _relativelocation_2))
  (Transformation|SetRelativeTransform (Variables|Default|GetAmmoMesh) (Math|Transform|MakeTransform (+ _relativelocation (Math|Vector|MakeVector _x _y (* (select (Variables|Default|GetMovingUp) 1.0 -1.0) DeltaSeconds 7.0))) (Math|Rotator|CombineRotators (Variables|/Script/Engine.SceneComponent|GetRelativeRotation _ammomesh) (Math|Rotator|MakeRotator 0.0 0.0 (* DeltaSeconds 1e+02))) (Variables|/Script/Engine.SceneComponent|GetRelativeScale3D (Variables|Default|GetAmmoMesh))) false false)
  (if (>= _z 1e+01)
    (Variables|Default|SetMovingUp false)
    (elif (<= _z 0.0)
      (Variables|Default|SetMovingUp true))))

(fn ConstructionScript)