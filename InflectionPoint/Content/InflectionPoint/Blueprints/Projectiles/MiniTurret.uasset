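; Short-lived mini turret that fires three shots at one-second intervals, then destroys itself.
; Each shot sphere-overlaps nearby BaseCharacters, picks the nearest living one and applies damage instantly, crediting the owner's instigator controller.
; Despite the SpawnProjectile name, shots are hitscan, shown by a sniper-trail beam emitter stretched from the turret mesh to the target.
; Damage taken by the turret is forwarded to its MortalityProvider.
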(event EventBeginPlay
  (Utilities|FlowControl|Delay 1.0)
  (CallFunction|SpawnProjectile 1e+01)
  (Utilities|FlowControl|Delay 1.0)
  (CallFunction|SpawnProjectile 1e+01)
  (Utilities|FlowControl|Delay 1.0)
  (CallFunction|SpawnProjectile 1e+01)
  (Actor|DestroyActor))

(event Collision|EventActorBeginOverlap
  (params (OtherActor :type Actor%20Object%20Reference)))

(event EventTick
  (params (DeltaSeconds :type Float%20%28single-precision%29)))

(event Game|Damage|EventAnyDamage
  (params (Damage :type Float%20%28single-precision%29) (DamageType :type Damage%20Type%20Object%20Reference) (InstigatedBy :type Controller%20Object%20Reference) (DamageCauser :type Actor%20Object%20Reference))
  (Class|MortalityProvider|TakeDamage (Variables|Default|GetMortalityProvider) Damage InstigatedBy DamageCauser))

(fn ConstructionScript)

(fn GetNearestCharacter
  (params (Array :type Array%20of%20Actor%20Object%20References))
  (for _array_element Array
    (bind _asbase_character (Utilities|Casting|CastToBaseCharacter _array_element))
    (bind _returnvalue (Class|BaseCharacter|IsAlive _asbase_character))
    (if (and _returnvalue (>= (LocalVariables|GetMinDist) (Transformation|GetDistanceTo _array_element self)))
      (LocalVariables|SetMinActor _array_element)
      (LocalVariables|SetMinDist (Transformation|GetDistanceTo _array_element self))))
  (return (LocalVariables|GetMinActor)))

(fn SpawnProjectile
  (params (Damage :type Float%20%28single-precision%29))
  (bind _staticmesh2 (Variables|Default|GetStaticMesh2))
  (bind _outactors (Collision|SphereOverlapActors (Transformation|GetActorLocation) 1e+03 (Utilities|Array|MakeArray "ObjectTypeQuery3") "/Script/InflectionPoint.BaseCharacter"))
  (bind _nearestcharacter (CallFunction|GetNearestCharacter _outactors))
  (Utilities|IsValid _nearestcharacter
    (:Is%20Valid
      (Game|Damage|ApplyDamage _nearestcharacter Damage (Game|GetInstigatorController (Components|GetOwner)) (Game|GetInstigator) "/Script/InflectionPoint.DefaultDamageType")
      (bind _returnvalue (Effects|SpawnEmitterAttached "/Game/InflectionPoint/Effects/SniperRifle_Trail.SniperRifle_Trail" _staticmesh2 "ShockBeamStart" "0, 0, 0" "0, 0, 0" "1.000000,1.000000,1.000000" "KeepWorldPosition"))
      (Effects|Components|ParticleSystem|SetVectorParameter _returnvalue "ShockBeamEnd" (Transformation|GetActorLocation _nearestcharacter))
      (Effects|Components|ParticleSystem|SetVectorParameter _returnvalue "ShockBeamStart" (Transformation|GetWorldLocation _staticmesh2)))))