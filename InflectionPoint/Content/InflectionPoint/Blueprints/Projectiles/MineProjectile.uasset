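; MineProjectile is a projectile actor that places a Mine where it lands.
; When its collision component hits something, it calls SpawnMine with the impact point and surface normal, then destroys itself.
; SpawnMine runs once, spawns the Mine only on the authority, rotates it to align with the surface normal, and passes on the projectile's owner and instigator.
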(event OnComponentHit(CollisionComp)
  (params (HitComponent :type Primitive%20Component%20Object%20Reference) (OtherActor :type Actor%20Object%20Reference) (OtherComp :type Primitive%20Component%20Object%20Reference) (NormalImpulse :type Vector :default "0, 0, 0") (Hit :type Hit%20Result%20Structure%20%28by%20ref%29))
  (bind (_bblockinghit _binitialoverlap _time _distance _location _impactpoint _normal) (Collision|BreakHitResult Hit))
  (CallFunction|SpawnMine _normal _impactpoint)
  (Actor|DestroyActor))

(fn ConstructionScript)

(fn SpawnMine
  (params (Normal :type Vector) (Location :type Vector))
  (if (not (Variables|Default|GetMineSpawned))
    (Variables|Default|SetMineSpawned true)
    (Networking|SwitchHasAuthority
      (:Authority
        (bind _returnvalue (Game|SpawnActorfromClass "/Game/InflectionPoint/Blueprints/Projectiles/Mine.Mine_C" (Math|Transform|MakeTransform Location (Math|Rotator|Delta(Rotator) (Math|Conversions|RotationFromXVector Normal) "90.000000, 0, 0")) "Undefined" (Components|GetOwner) (Variables|Default|GetInstigator)))
        (return _returnvalue)))))