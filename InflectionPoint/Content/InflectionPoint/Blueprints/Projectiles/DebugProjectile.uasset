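; DebugProjectile is a projectile Blueprint that visualizes its flight result for debugging.
; On BeginPlay it records its start position and prints the game time.
; On Hit it prints the colliding component's transform, draws a long-lived point and a straight line from the start to that component's location, then destroys itself.
; Any destruction spawns a Water_Splash actor at its transform.
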(event Collision|EventHit
  (params (MyComp :type Primitive%20Component%20Object%20Reference) (Other :type Actor%20Object%20Reference) (OtherComp :type Primitive%20Component%20Object%20Reference) (bSelfMoved :type Boolean) (HitLocation :type Vector :default "0, 0, 0") (HitNormal :type Vector :default "0, 0, 0") (NormalImpulse :type Vector :default "0, 0, 0") (Hit :type Hit%20Result%20Structure%20%28by%20ref%29))
  (bind _returnvalue (Transformation|GetWorldLocation MyComp))
  ;[1 1 1] Draw debug line
  (if true
    (Development|PrintText (Utilities|Text|ToText(String) (Transformation|GetWorldTransform MyComp)))
    (Rendering|Debug|DrawDebugPoint _returnvalue 1e+01 "(R=0.995000,G=0.413286,B=0.000000,A=1.000000)" 9347856.0)
    (Rendering|Debug|DrawDebugLine (Variables|Default|GetStartPos) _returnvalue "(R=1.000000,G=0.604754,B=0.000000,A=1.000000)" 3265467547.0 1.0)
    (Actor|DestroyActor)))

(event EventBeginPlay
  ;[1 1 1] Init
  (Variables|Default|SetStartPos (Transformation|GetActorLocation))
  (Development|PrintString (Class|KismetStringLibrary|TimeSecondstoString (Utilities|Time|GetTimeSeconds)) true true "(R=0.000000,G=0.660000,B=1.000000,A=1.000000)" 34234.0))

(event EventDestroyed
  ;[1 1 1] Spawn Splash
  (Game|SpawnActorfromClass "/Game/InflectionPoint/Blueprints/Effects/Water_Splash.Water_Splash_C" (Transformation|GetActorTransform) "Undefined" 0 0))

(fn ConstructionScript)