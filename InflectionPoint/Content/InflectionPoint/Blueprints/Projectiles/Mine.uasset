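; Mine is a placed explosive actor that detonates when a character touches it or when it is destroyed by damage.
; A box overlap with any BaseCharacter, or the MortalityProvider's death event, spawns a MineExplosion at the ExplosionSpawn point and destroys the mine.
; Incoming damage is forwarded to MortalityProvider, and the explosion inherits the mine's owner and instigator.
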(event OnDeath(MortalityProvider)
  (params (KillingPlayer :type Controller%20Object%20Reference) (DamageCauser :type Actor%20Object%20Reference))
  (Game|SpawnActorfromClass "/Game/InflectionPoint/Blueprints/Explosions/MineExplosion.MineExplosion_C" (Transformation|GetWorldTransform (Variables|Default|GetExplosionSpawn)) "AlwaysSpawn" (Components|GetOwner) (Game|GetInstigator))
  (Actor|DestroyActor))

(event OnComponentBeginOverlap(Box)
  (params (OverlappedComponent :type Primitive%20Component%20Object%20Reference) (OtherActor :type Actor%20Object%20Reference) (OtherComp :type Primitive%20Component%20Object%20Reference) (OtherBodyIndex :type Integer) (bFromSweep :type Boolean) (SweepResult :type Hit%20Result%20Structure%20%28by%20ref%29))
  (bind _asbase_character (Utilities|Casting|CastToBaseCharacter OtherActor))
  (Utilities|IsValid _asbase_character
    (:Is%20Valid
      (Game|SpawnActorfromClass "/Game/InflectionPoint/Blueprints/Explosions/MineExplosion.MineExplosion_C" (Transformation|GetWorldTransform (Variables|Default|GetExplosionSpawn)) "AlwaysSpawn" (Components|GetOwner) (Game|GetInstigator))
      (Actor|DestroyActor))))

(event EventBeginPlay)

(event Collision|EventActorBeginOverlap
  (params (OtherActor :type Actor%20Object%20Reference)))

(event EventTick
  (params (DeltaSeconds :type Float%20%28single-precision%29)))

(event Game|Damage|EventAnyDamage
  (params (Damage :type Float%20%28single-precision%29) (DamageType :type Damage%20Type%20Object%20Reference) (InstigatedBy :type Controller%20Object%20Reference) (DamageCauser :type Actor%20Object%20Reference))
  (Class|MortalityProvider|TakeDamage (Variables|Default|GetMortalityProvider) Damage InstigatedBy DamageCauser))

(fn ConstructionScript)