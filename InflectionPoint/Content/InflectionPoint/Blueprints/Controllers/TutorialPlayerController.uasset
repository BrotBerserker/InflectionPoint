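; Player controller for the tutorial that lets forward movement, jump and sprint be switched on and off individually.
; Gates controlled by Enable/Disable events pass input to the controlled BaseCharacter and log it to its PlayerStateRecorder, with only positive forward axis values accepted.
; It overrides the parent's left-click spectator switching and BeginPlay to avoid an input mode change, caching the pawn and adding an in-game menu widget instead.
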(event Custom|DisableForwardMovement
  (Utilities|FlowControl|Gate false) ; enters at Close
)

(event Custom|EnableJump
  (Utilities|FlowControl|Gate true) ; enters at Open
)

(event Custom|EnableSprint
  (bind _recorder (Variables|Default|GetRecorder))
  (bind _controlledcharacter (Variables|Default|GetControlledCharacter))
  (Utilities|FlowControl|Sequence
    (:then_0
      (Utilities|FlowControl|Gate true) ; enters at Open
    )
    (:then_1
      (Utilities|FlowControl|Gate true) ; enters at Open
    )))

(event Custom|EnableForwardMovement
  (Utilities|FlowControl|Gate false) ; enters at Open
)

(event Custom|DisableJump
  (Utilities|FlowControl|Gate true) ; enters at Close
)

(event Custom|DisableSprint
  (bind _recorder (Variables|Default|GetRecorder))
  (bind _controlledcharacter (Variables|Default|GetControlledCharacter))
  (Utilities|FlowControl|Sequence
    (:then_0
      (Utilities|FlowControl|Gate true) ; enters at Close
    )
    (:then_1
      (Utilities|FlowControl|Gate true) ; enters at Close
    )))

(event EventBeginPlay
  ;[1 1 1] Disable parent's begin play to avoid change of input mode
  (CallFunction|UpdateControlledPawn (Pawn|GetControlledPawn))
  (bind _returnvalue (UserInterface|CreateWidget "/Game/InflectionPoint/UI/Menus/IngameMenu.IngameMenu_C"))
  (bind _output_get (Variables|Default|SetIngameMenu _returnvalue))
  (UserInterface|Viewport|AddtoViewport _output_get 1))

(event Input|ActionEvents|InputActionSprint
  (params (Key :type Key%20Structure))
  (bind _recorder (Variables|Default|GetRecorder))
  (bind _controlledcharacter (Variables|Default|GetControlledCharacter))
  (:Pressed
    (Utilities|FlowControl|Gate true
      (:Exit
        (Class|BaseCharacter|EnableSprint _controlledcharacter)
        (Class|PlayerStateRecorder|RecordKey _recorder "Sprint" "IE_Pressed"))))
  (:Released
    (Utilities|FlowControl|Gate true
      (:Exit
        (Class|BaseCharacter|DisableSprint _controlledcharacter)
        (Class|PlayerStateRecorder|RecordKey _recorder "Sprint" "IE_Released")))))

(event Input|ActionEvents|InputActionJump
  (params (Key :type Key%20Structure))
  (:Pressed
    (Utilities|FlowControl|Gate true
      (:Exit
        (Character|Jump (Variables|Default|GetControlledCharacter))
        (Class|PlayerStateRecorder|RecordKey (Variables|Default|GetRecorder) "Jump" "IE_Pressed")))))

(event Input|AxisEvents|InputAxisMoveForward
  (params (AxisValue :type Float%20%28single-precision%29))
  (Utilities|FlowControl|Gate false
    (:Exit
      (if (> AxisValue 0.0)
        (Class|BaseCharacter|MoveForward (Variables|Default|GetControlledCharacter) AxisValue)
        (Class|PlayerStateRecorder|RecordMoveForward (Variables|Default|GetRecorder) AxisValue)))))

(event Input|MouseEvents|LeftMouseButton
  (params (Key :type Key%20Structure))
  ;[1 1 1] Disable spectator switching
  (:Pressed
    (Utilities|FlowControl|Delay 0.0) ; Dummy code to override parent implementation
  ))

(fn ConstructionScript
  (|CallParentFunction))

(fn UpdateControlledPawn
  (params (Object :type Object%20Object%20Reference))
  (bind _asbase_character (Utilities|Casting|CastToBaseCharacter Object))
  (bind _output_get (Variables|Default|SetControlledCharacter _asbase_character))
  (Variables|Default|SetRecorder (Actor|GetComponentbyClass _output_get "/Script/InflectionPoint.PlayerStateRecorder")))