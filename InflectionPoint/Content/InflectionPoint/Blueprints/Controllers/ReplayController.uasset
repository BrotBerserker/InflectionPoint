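; AI controller for replay characters that can take over the pawn with bot AI once its replay finishes.
; On possess it binds to the pawn's damage, death and replay-finished events.
; If takeover is enabled, it shows a takeover indicator, waits, then runs the bot behavior tree if still alive, storing the current location as home.
; Damage records the instigator's pawn on the blackboard, and death stops movement and tree logic.
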(event Custom|ReplayFinished
  (bind _returnvalue (Math|Float|MakeLiteralFloat 5.0))
  ;[1 1 1] Start AI Controlling
  (bind _asreplay_character (Utilities|Casting|CastToReplayCharacter (Pawn|GetControlledPawn)))
  (if (Variables|/Script/InflectionPoint.ReplayCharacterBase|GetAITakeoverAfterReplayEnd _asreplay_character)
    (Default|ShowAITakingControll _asreplay_character _returnvalue)
    (Utilities|FlowControl|Delay _returnvalue)
    (bind _returnvalue_2 (Class|BaseCharacter|IsAlive _asreplay_character))
    (if _returnvalue_2
      (CallFunction|RunBehaviourTree))))

(event Custom|ReplayDeath
  (params (KillingPlayer :type Controller%20Object%20Reference) (DamageCauser :type Actor%20Object%20Reference))
  ;[1 1 1] StopTree OnDeath
  (CallFunction|StopBehaviorTree))

(event Custom|DamageTaken
  (params (DamagedActor :type Actor%20Object%20Reference) (Damage :type Float%20%28single-precision%29) (DamageType :type Damage%20Type%20Object%20Reference) (InstigatedBy :type Controller%20Object%20Reference) (DamageCauser :type Actor%20Object%20Reference))
  ;[1 1 1] Update DamageCauser Blackboardkey
  (CallFunction|UpdateLastDamageCauseronBlackboard InstigatedBy))

(event EventOnPossess
  (params (PossessedPawn :type Pawn%20Object%20Reference))
  (bind _asreplay_character_base (Utilities|Casting|CastToReplayCharacterBase PossessedPawn))
  (Utilities|FlowControl|Sequence
    (:then_0
      ;[1 1 1] Update DamageCauser Blackboardkey
      (EventDispatchers|BindEventtoOnTakeAnyDamage (Pawn|GetControlledPawn) (delegate Custom|DamageTaken)))
    (:then_1
      ;[1 1 1] StopTree OnDeath
      (EventDispatchers|BindEventtoOnDeath (Variables|/Script/InflectionPoint.BaseCharacter|GetMortalityProvider _asreplay_character_base) (delegate Custom|ReplayDeath)))
    (:then_2
      ;[1 1 1] Start AI Controlling
      (EventDispatchers|BindEventtoOnFinishedReplaying _asreplay_character_base (delegate Custom|ReplayFinished)))))

(fn ConstructionScript)

(fn UpdateLastDamageCauseronBlackboard
  (params (DamageCauser :type Controller%20Object%20Reference))
  (bind _returnvalue (AI|GetBlackboard 0))
  (Utilities|IsValid _returnvalue
    (:Is%20Valid
      (AI|Components|Blackboard|SetValueasObject _returnvalue (Variables|Default|GetLastDamageCauser) (Pawn|GetControlledPawn DamageCauser)))))

(fn StopBehaviorTree
  (bind _braincomponent (Variables|Default|GetBrainComponent))
  (AI|Navigation|StopMovement)
  (Utilities|IsValid _braincomponent
    (:Is%20Valid
      (AI|Logic|StopLogic _braincomponent "Death"))))

(fn RunBehaviourTree
  (bind _blackboardcomponent (Class|AIController|UseBlackboard "/Game/InflectionPoint/Blueprints/AI/BotBlackboard.BotBlackboard"))
  (AI|Components|Blackboard|SetValueasVector _blackboardcomponent (Variables|Default|GetHomeLocation) (Transformation|GetActorLocation (Pawn|GetControlledPawn)))
  (AI|RunBehaviorTree "/Game/InflectionPoint/Blueprints/AI/BotBehaviourTree.BotBehaviourTree"))