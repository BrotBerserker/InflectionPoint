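; Player controller for Inflection Point that creates the ingame menu and drives the HUD through rounds, countdowns, damage, kills, score and death.
; Round and character changes set HUD views, locking character input after round zero.
; Input toggles the menu, scoreboard and aim/X-ray post-processing, and lets dead players cycle spectated characters through the server.
; A per-tick line trace shows teammate name tags, while identity checks separate players from their replays.
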(event Custom|CharacterChanged
  (params (Character :type Player%20Character%20Object%20Reference))
  ;[1 1 1] Update Mortality Provider when controlled character changes, switch to Ingame View if round 0
  (bind _inflectionpointhud (CallFunction|GetInitializedInflectionPointHUDReference))
  (Utilities|IsValid _inflectionpointhud
    (:Is%20Valid
      (Default|SetMortalityProvider _inflectionpointhud (Actor|GetComponentbyClass Character "/Script/InflectionPoint.MortalityProvider"))
      (if (== (Variables|Default|GetCurrentRound) 0)
        (Default|SwitchtoIngameView _inflectionpointhud)
        (else
          (Input|DisableInput Character self)))
      (Variables|/Script/Engine.PostProcessComponent|SetbEnabled (Variables|Default|GetPostProcessXRay) false)
      (Variables|/Script/Engine.PostProcessComponent|SetbEnabled (Variables|Default|GetPostProcessAim) false))))

(event Custom|ClientShowDamageDealt
  ;[1 1 1] Display dealt/received Damage in HUD
  (Default|ShowDamageDealt (Variables|Default|GetInflectionPointHUD)))

(event Custom|ClientShowSpectatorViewSwitched
  (params (CharacterInfo :type Character%20Info%20Structure))
  ;[1 1 1] Update HUD when spectated character switches
  (bind _output_get (Variables|Default|SetSpectatedCharacter CharacterInfo))
  (Default|SetSpectatingCharacterInformation (Variables|Default|GetInflectionPointHUD) _output_get)
  (Default|SwitchtoSpectatorView (Variables|Default|GetInflectionPointHUD)))

(event Custom|DirectionalDamageReceived
  (params (Direction :type Vector) (Damage :type Float%20%28single-precision%29))
  ;[1 1 1] Display dealt/received Damage in HUD
  (Default|ShowDirectionalDamageRecieved (Variables|Default|GetInflectionPointHUD) Direction Damage))

(event EventBeginPlay
  ;[1 1 1] Initialize HUD and Ingame Menu, set Input Mode
  (Input|SetInputModeGameOnly self)
  (if (Pawn|IsLocalController)
    (bind _returnvalue (UserInterface|CreateWidget "/Game/InflectionPoint/UI/Menus/IngameMenu.IngameMenu_C"))
    (bind _output_get (Variables|Default|SetIngameMenu _returnvalue))
    (UserInterface|Viewport|AddtoViewport _output_get 1)))

(event EventOnCountdownUpdate
  (params (number :type Integer))
  (bind _inflectionpointhud (Variables|Default|GetInflectionPointHUD))
  ;[1 1 1] Display Countdown on HUD
  (Default|ShowRemainingTimetoStart _inflectionpointhud number)
  (if (== number 0)
    (Utilities|FlowControl|Delay 1.0) ; Wait for countdown animation to finish
    (Default|SwitchtoIngameView _inflectionpointhud)))

(event EventTick
  (params (DeltaSeconds :type Float%20%28single-precision%29))
  ;[1 1 1] Update displayed name tag in Tick
  (if (Pawn|IsLocalPlayerController)
    (CallFunction|UpdateDisplayedCharacterNameTag)))

(event EventOnKillInfoAdded
  (params (KilledInfo :type Character%20Info%20Structure) (killedScoreChange :type Float%20%28single-precision%29) (KillerInfo :type Character%20Info%20Structure) (killerScoreChange :type Float%20%28single-precision%29) (WeaponImage :type Texture%202D%20Object%20Reference))
  ;[1 1 1] Display Kill Info on HUD
  (bind _out (CallFunction|GetOwnScoreChange KilledInfo killedScoreChange KillerInfo killerScoreChange))
  (Default|ShowKill (Variables|Default|GetInflectionPointHUD) WeaponImage KillerInfo KilledInfo _out)
  (Utilities|IsOwnCharacter KilledInfo
    (:true
      (Default|SwitchtoDeathView (Variables|Default|GetInflectionPointHUD)))
    (:false
      _))
  (Utilities|IsSelfAlive
    (:False
      (Utilities|IsSameCharacter KilledInfo (Variables|Default|GetSpectatedCharacter)
        (:True
          (Class|PlayerControllerBase|ServerSwitchSpectatedCharacter))))))

(event EventDamageDealt
  ;[1 1 1] Display dealt/received Damage in HUD
  (CallFunction|ClientShowDamageDealt))

(event EventOnRoundStarted
  (params (Round :type Integer))
  ;[1 1 1] Update HUD when Round starts
  (bind _output_get (Variables|Default|SetCurrentRound Round))
  (bind _inflectionpointhud (CallFunction|GetInitializedInflectionPointHUDReference))
  (if (not (== _output_get 0))
    (Default|SwitchtoCountdownView _inflectionpointhud)))

(event EventSpectatedCharacterSwitched
  (params (newCharacter :type Base%20Character%20Object%20Reference) (newCharacterInfo :type Character%20Info%20Structure))
  ;[1 1 1] Update HUD when spectated character switches
  (CallFunction|ClientShowSpectatorViewSwitched newCharacterInfo))

(event Input|ActionEvents|InputActionBack
  (params (Key :type Key%20Structure :default "AnyKey"))
  ;[1 1 1] Show/Hide Ingame Menu
  (:Pressed
    (if (Widget|IsVisible (Variables|Default|GetIngameMenu))
      (Default|Hide (Variables|Default|GetIngameMenu))
      (else
        (Default|Show (Variables|Default|GetIngameMenu))))))

(event Input|ActionEvents|InputActionAim
  (params (Key :type Key%20Structure :default "AnyKey"))
  (bind _postprocessaim (Variables|Default|GetPostProcessAim))
  ;[1 1 1] Hide crosshair when aiming
  (:Pressed
    (Utilities|IsSelfAlive
      (:True
        (Variables|/Script/Engine.PostProcessComponent|SetbEnabled _postprocessaim true))))
  (:Released
    (Utilities|IsSelfAlive
      (:True
        (Variables|/Script/Engine.PostProcessComponent|SetbEnabled _postprocessaim false)))))

(event Input|ActionEvents|InputActionXRayView
  (params (Key :type Key%20Structure :default "AnyKey"))
  (bind _postprocessxray (Variables|Default|GetPostProcessXRay))
  ;[1 1 1] Enable/Disable XRay View
  (:Pressed
    (bind _output_get (Variables|/Script/Engine.PostProcessComponent|SetbEnabled _postprocessxray (not (Variables|/Script/Engine.PostProcessComponent|GetbEnabled _postprocessxray))))
    (Audio|PlaySound2D "/Game/Sounds/XRay/KlickSound.KlickSound")
    (Default|SetXRaySkillActive (Variables|Default|GetInflectionPointHUD) _output_get)))

(event Input|KeyboardEvents|Tab
  (params (Key :type Key%20Structure :default "AnyKey"))
  (bind _inflectionpointhud (Variables|Default|GetInflectionPointHUD))
  ;[1 1 1] Show Scoreboard when pressing Tab
  (:Pressed
    (Default|ShowScore _inflectionpointhud))
  (:Released
    (Default|HideScore _inflectionpointhud)))

(event Input|MouseEvents|LeftMouseButton
  (params (Key :type Key%20Structure :default "AnyKey"))
  ;[1 1 1] Switch spectated character
  (:Pressed
    (Utilities|IsSelfAlive
      (:False
        (Class|PlayerControllerBase|ServerSwitchSpectatedCharacter)))))

(fn ConstructionScript)

(fn GetInitializedInflectionPointHUDReference
  (Utilities|IsValid (Variables|Default|GetInflectionPointHUD)
    (:Is%20Valid
      (return (Variables|Default|GetInflectionPointHUD)))
    (:Is%20Not%20Valid
      (bind _asinflection_point_hud (Utilities|Casting|CastToInflectionPointHUD (HUD|GetHUD)))
      (bind _output_get (Variables|Default|SetInflectionPointHUD _asinflection_point_hud))
      (return _output_get))))

(fn GetOwnScoreChange
  (params (Killed :type Character%20Info%20Structure) (KilledScore :type Float%20%28single-precision%29) (Killer :type Character%20Info%20Structure) (KillerScore :type Float%20%28single-precision%29))
  (Utilities|IsOwnCharacterorReplay Killer
    (:true
      (LocalVariables|SetScoreChange (+ (LocalVariables|GetScoreChange) KillerScore)))
    (:false
      _))
  (Utilities|IsOwnCharacterorReplay Killed
    (:true
      (LocalVariables|SetScoreChange (+ (LocalVariables|GetScoreChange) KilledScore)))
    (:false
      _))
  (return (LocalVariables|GetScoreChange)))

(fn UpdateDisplayedCharacterNameTag
  (bind (_start _end) (Utilities|GetLineTraceLocations))
  (bind _inflectionpointhud (Variables|Default|GetInflectionPointHUD))
  (bind (_outhit _returnvalue) (Collision|LineTraceByChannel _start _end "TraceTypeQuery3" false (Utilities|Array|MakeArray (Pawn|GetControlledPawn)) "None" true "(R=0.075611,G=0.000000,B=1.000000,A=1.000000)"))
  (if _returnvalue
    (Utilities|IsValid (Actor|GetComponentbyClass (.HitActor (Collision|BreakHitResult _outhit)) "/Script/InflectionPoint.CharacterInfoProvider")
      (:Is%20Valid
        (bind _returnvalue_2 (Class|CharacterInfoProvider|GetCharacterInfo (Actor|GetComponentbyClass (.HitActor (Collision|BreakHitResult _outhit)) "/Script/InflectionPoint.CharacterInfoProvider")))
        (Utilities|CharacterIsinMyTeam _returnvalue_2
          (:true
            (bind _inflectionpointhud_2 (CallFunction|GetInitializedInflectionPointHUDReference))
            (Default|ShowCharacterNameTag _inflectionpointhud_2 _returnvalue_2 (.HitActor (Collision|BreakHitResult _outhit)))))))
    (else
      (Utilities|IsValid _inflectionpointhud
        (:Is%20Valid
          (Default|ShowCharacterNameTag _inflectionpointhud))))))