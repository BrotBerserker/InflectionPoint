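; AI controller for tutorial enemies that switches between a scripted tutorial behavior and regular bot behavior.
; StartTutorialBotting, if the controlled BaseCharacter is alive, loads the tutorial blackboard, writes a target location and target actor into it, then runs the tutorial enemy behavior tree.
; StartRealBotting swaps in the standard bot blackboard and behavior tree without an alive check.
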(event Custom|StartTutorialBotting
  (params (VectorValue :type Vector) (ObjectValue :type Object%20Object%20Reference))
  (bind _asbase_character (Utilities|Casting|CastToBaseCharacter (Pawn|GetControlledPawn)))
  (bind _returnvalue (Class|BaseCharacter|IsAlive _asbase_character))
  (if _returnvalue
    (Class|AIController|UseBlackboard "/Game/InflectionPoint/Blueprints/AI/TutorialEnemyBlackboard.TutorialEnemyBlackboard")
    (AI|Components|Blackboard|SetValueasVector (AI|GetBlackboard 0) (Utilities|Name|MakeLiteralName "TargetLocation") VectorValue)
    (AI|Components|Blackboard|SetValueasObject (AI|GetBlackboard 0) (Utilities|Name|MakeLiteralName "TargetActor") ObjectValue)
    (AI|RunBehaviorTree "/Game/InflectionPoint/Blueprints/AI/TutorialEnemyBehaviour.TutorialEnemyBehaviour")))

(event Custom|StartRealBotting
  (Class|AIController|UseBlackboard "/Game/InflectionPoint/Blueprints/AI/BotBlackboard.BotBlackboard")
  (AI|RunBehaviorTree "/Game/InflectionPoint/Blueprints/AI/BotBehaviourTree.BotBehaviourTree"))

(event EventBeginPlay)

(fn ConstructionScript)